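; Game mode that runs endless enemy waves and tracks the score.
; Tick watches for zero living enemies, then grows the enemy total (except every fifth wave), fills the SpawnerController and starts the next wave after a delay.
; Enemies are picked randomly per tier, with the tier ceiling derived from wave number / 5 and fixed percentage shares based on distance from that ceiling.
; Wave progress is reported through debug prints.
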(event Custom|UpdateScore
  (params (Score%20Change :type Integer))
  (Variables|Default|Setscore (+ (Variables|Default|Getscore) Score%20Change)))

(event Custom|newWave
  (bind _result (Math|Integer|IncrementInt (Variables|Default|GetwaveNumber))
    (:%20%20
      (bind _output_get (Variables|Default|SetwaveNumber _result))
      (Variables|Default|SetenemiesAliveInWave (Variables|Default|GettotalEnemiesInWave))
      (Actor|Tick|SetActorTickEnabled true)
      (Default|NewWave (Variables|Default|GetspawnerController))
      (Development|PrintString (Utilities|String|Append (Utilities|String|MakeLiteralString "WAVE N°") (Utilities|String|MakeLiteralString (Utilities|String|ToString(Integer) _output_get))) true true "(R=0.505000,G=0.000000,B=0.353093,A=1.000000)")
      (Development|PrintString (Utilities|String|Append (Utilities|String|MakeLiteralString "Enemies in wave : ") (Utilities|String|MakeLiteralString (Utilities|String|ToString(Integer) (Variables|Default|GettotalEnemiesInWave)))) true true "(R=0.315000,G=0.000000,B=0.305475,A=1.000000)"))))

(event Custom|WaveFinished
  (CallFunction|IncreaseTotalEnemiesinWave 1)
  (bind _selectedenemies (CallFunction|SelectEnemiesforNextWave))
  (for _array_element _selectedenemies
    (Utilities|Array|Add (Variables|Default|GettestTimers) 2))
  (Default|FillEnemySpawners (Variables|Default|GetspawnerController) _selectedenemies (Variables|Default|GettestTimers))
  (Utilities|FlowControl|Delay (Math|Conversions|ToFloat(Integer) (Variables|Default|GettimeBetweenWaves)))
  (CallFunction|NewWave)
  (Development|PrintString "New wave" true true "(R=0.273015,G=0.000000,B=0.335000,A=1.000000)"))

(event EventBeginPlay
  (CallFunction|NewWave)
  (bind _outactors (Actor|GetAllActorsOfClass "/Game/Ennemies/SpawnerController.SpawnerController_C"))
  (Variables|Default|SetspawnerController (Utilities|Array|Get(acopy) _outactors)))

(event EventTick
  (params (DeltaSeconds :type Float%20%28single-precision%29))
  (if (== (Variables|Default|GetenemiesAliveInWave) 0)
    (CallFunction|WaveFinished)
    (Actor|Tick|SetActorTickEnabled false)
    (Development|PrintString "Wave finished" true true "(R=0.273307,G=0.000000,B=0.280000,A=1.000000)")))

(fn ConstructionScript)

(fn IncreaseTotalEnemiesinWave
  (params (Value :type Integer))
  (if (not (== (Math|Integer|%(Integer) (Variables|Default|GetwaveNumber) 5) 0))
    (Variables|Default|SettotalEnemiesInWave (+ (Variables|Default|GettotalEnemiesInWave) Value))))

(fn SelectRandomEnemyinTier
  (params (Tier :type Tier%20Structure))
  (bind _enemies (Utilities|Struct|BreakTier Tier))
  (bind _output_get (LocalVariables|SetTierLength (Utilities|Array|Length _enemies)))
  (return (Utilities|Array|Get(acopy) _enemies (Math|Random|RandomInteger _output_get))))

(fn SelectRandomEnemiesinTier
  (params (Tier :type Tier%20Structure) (Number :type Integer) (Additional%20Enemies :type Integer))
  (for _index (range 0 (+ Number (Math|Random|RandomInteger Additional%20Enemies)))
    (bind _selected_enemy (CallFunction|SelectRandomEnemyinTier Tier))
    (Utilities|Array|Add (LocalVariables|GetResult) _selected_enemy)
    (Development|PrintString "Enemy added"))
  (return (LocalVariables|GetResult)))

(fn SelectEnemiesforNextWave
  (bind _maxtier (CallFunction|MaxTier))
  (bind _output_get (LocalVariables|SetmaximumTier _maxtier))
  (for _index (range 0 _output_get)
    ;[1 1 1] Loop : for each Tier
    (bind _result (Math|Integer|IncrementInt (LocalVariables|GetcurrentTier))
      (:%20%20
        (bind _output_get_2 (LocalVariables|SetcurrentTier _result))
        (bind _numberofenemies (CallFunction|NumberOfEnemiesPerTier (LocalVariables|GetmaximumTier) _output_get_2 (Variables|Default|GettotalEnemiesInWave)))
        (bind _selected_enemies (CallFunction|SelectRandomEnemiesinTier (Utilities|Array|Get(acopy) (Variables|Default|GetTiers) _index) _numberofenemies))
        (Utilities|Array|AppendArray (LocalVariables|GetEnemies) _selected_enemies))))
  (return (LocalVariables|GetEnemies)))

(fn MaxTier
  (return (/ (Variables|Default|GetwaveNumber) 5)))

(fn NumberOfEnemiesPerTier
  (params (maxTier :type Integer) (currentTier :type Integer) (totalEnemies :type Integer))
  (LocalVariables|SettotalEnemiesLocal totalEnemies)
  (switch int (- maxTier currentTier)
    (:Default
      (LocalVariables|Setpercentage 0.0))
    (:0
      (LocalVariables|Setpercentage 0.05))
    (:1
      (LocalVariables|Setpercentage 0.15))
    (:2
      (LocalVariables|Setpercentage 0.3))
    (:3
      (LocalVariables|Setpercentage 0.5)))
  (return (Math|Float|Ceil (* (LocalVariables|GettotalEnemiesLocal) (LocalVariables|Getpercentage)))))